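; Spawn volume actor that places pickup-style items (Bino, Bone, Key, Camera, Diploma) at random points within its bounds.
; BeginPlay starts a near-immediate timer on SpawnNewItem, repeating according to the Looping variable.
; SpawnNewItem recursively retries while a box overlap finds a NoSpawnVolume at the random point, then spawns all five items.
; Only the first item's location gets that overlap check; the other four use fresh, unchecked random points.
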(event Custom|SpawnNewItem
  (bind _volume (Variables|Default|GetVolume))
  (bind (_origin _boxextent) (Collision|GetComponentBounds _volume))
  (bind (_x _y _z) (Math|Vector|BreakVector _origin))
  (bind (_x_2 _y_2) (Math|Vector|BreakVector _boxextent))
  (bind _returnvalue (- _x _x_2))
  (bind _returnvalue_2 (- _y _y_2))
  (bind _returnvalue_3 (+ _x _x_2))
  (bind _returnvalue_4 (+ _y _y_2))
  (bind _returnvalue_5 (Math|Random|RandomFloatinRange _returnvalue _returnvalue_3))
  (bind _returnvalue_6 (Math|Random|RandomFloatinRange _returnvalue_2 _returnvalue_4))
  (bind _returnvalue_7 (Math|Vector|MakeVector _returnvalue_5 _returnvalue_6 _z))
  (Variables|Default|SetRandomLocation _returnvalue_7)
  (bind _returnvalue_8 (Collision|BoxOverlapActors (Variables|Default|GetRandomLocation) "32.000000,32.000000,32.000000" (Utilities|Array|MakeArray "ObjectTypeQuery2") "/Game/BluePrints/Spawning/NoSpawnVolume.NoSpawnVolume_C" :!class /Script/Engine.KismetSystemLibrary))
  (if _returnvalue_8
    (CallFunction|SpawnNewItem)
    (else
      (Game|SpawnActorfromClass "/Game/BluePrints/Items/Bino.Bino_C" (Math|Conversions|ToTransform(Vector) (Variables|Default|GetRandomLocation)) "Undefined" 0 0)
      (Variables|Default|SetRandomLocation _returnvalue_7)
      (Game|SpawnActorfromClass "/Game/BluePrints/Items/Bone.Bone_C" (Math|Conversions|ToTransform(Vector) (Variables|Default|GetRandomLocation)) "Undefined" 0 0)
      (Variables|Default|SetRandomLocation _returnvalue_7)
      (Game|SpawnActorfromClass "/Game/BluePrints/Items/Key.Key_C" (Math|Conversions|ToTransform(Vector) (Variables|Default|GetRandomLocation)) "Undefined" 0 0)
      (Variables|Default|SetRandomLocation _returnvalue_7)
      (Game|SpawnActorfromClass "/Game/BluePrints/Items/Camera.Camera_C" (Math|Conversions|ToTransform(Vector) (Variables|Default|GetRandomLocation)) "Undefined" 0 0)
      (Variables|Default|SetRandomLocation _returnvalue_7)
      (Game|SpawnActorfromClass "/Game/BluePrints/Items/Diploma.Diploma_C" (Math|Conversions|ToTransform(Vector) (Variables|Default|GetRandomLocation)) "Undefined" 0 0))))

(event EventBeginPlay
  (Utilities|Time|SetTimerbyFunctionName 0 "SpawnNewItem" 0.01 (Math|Conversions|ToBoolean(Integer) (stale _output_get))))

(fn ConstructionScript)